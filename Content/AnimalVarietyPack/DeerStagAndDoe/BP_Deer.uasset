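; BP_Deer is a deer with simple wandering and fleeing behavior driven by an event loop in its own graph.
; DecideNextAction picks a fast run when ShouldRun is set, otherwise a slow roam unless tired or hungry.
; Both moves use AI MoveTo toward random reachable points and re-decide only on success, with running skipping the random idle delay.
; Nothing here sets the state flags, and fleeing ignores threat direction.
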(event `self.ReceiveBeginPlay`
  (`self.Decide Next Action` false))

(event `Decide Next Action`
  (params (`SkipDelay?` :type Boolean))
  (if (not `SkipDelay?`)
    (`KismetSystemLibrary.Delay` (`KismetMathLibrary.RandomFloatInRange` 1.0 8.0)))
  (if (`self.Should Run?`)
    (`self.Run Away`)
    (elif (`self.Is Tired?`)
      _
      (elif (not (`self.Is Hungry?`))
        (`self.Random Roam`)))))

(event `Random Roam`
  ;[1 1 1] Random roam
  (set `CharacterMovementComponent.MaxWalkSpeed` 200.0 (`self.CharacterMovement`))
  (`|AIMoveTo` self (`NavigationSystemV1.K2_GetRandomReachablePointInRadius` (`self.K2_GetActorLocation`) 1500.0 null null) null
    (:`OnSuccess`
      (`self.Decide Next Action` false))))

(event `Run Away`
  ;[1 1 1] Run away
  (set `CharacterMovementComponent.MaxWalkSpeed` 700.0 (`self.CharacterMovement`))
  (`|AIMoveTo` self (`NavigationSystemV1.K2_GetRandomReachablePointInRadius` (`self.K2_GetActorLocation`) (`KismetMathLibrary.RandomFloatInRange` 1000.0 3000.0) null null) null
    (:`OnSuccess`
      (`self.Decide Next Action` true))))

(fn `UserConstructionScript`)