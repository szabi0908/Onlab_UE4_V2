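; Wolf animal Blueprint that roams randomly, flees once hurt and drops meat when killed.
; DecideNextAction loops through AIMoveTo: slow delayed roaming with timed health regeneration, or fast continuous fleeing once ShouldRun is set.
; Projectile hits feed TakeDamage, which either triggers a hit reaction and flight, or death, a BP_Meat spawn and delayed destruction.
; PlayAnimation and StopAnimation are empty here, and ShouldRun is never reset.
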(event `Take Damage`
  (bind _charactermovement (`self.CharacterMovement`))
  ;[1 1 1] Tage Damage
  (if (not (`self.Is Dead?`))
    (bind _output_get (set `self.Health` (`KismetMathLibrary.Clamp` (- (`self.Health`) (`self.Damage`)) 0 (`self.MaxHealth`))))
    (if (== _output_get 0)
      (`MovementComponent.StopMovementImmediately` _charactermovement)
      (set `self.Is Dead?` true)
      (`CharacterMovementComponent.DisableMovement` (`self.CharacterMovement`))
      (`self.Play Animation` "/Game/AnimalVarietyPack/Wolf/Animations/ANIM_Wolf_Death.ANIM_Wolf_Death")
      (`|SpawnActorFromClass` "/Game/Blueprints/BP_Meat.BP_Meat_C" (`KismetMathLibrary.MakeTransform` (- (`self.K2_GetActorLocation`) (150.0 0.0 85.0))) "Undefined" "OverrideRootScale" null null)
      (`KismetSystemLibrary.Delay` (`KismetMathLibrary.RandomFloatInRange` 5.0 10.0))
      (`self.K2_DestroyActor`)
      (else
        (`MovementComponent.StopMovementImmediately` _charactermovement)
        (`self.Play Animation` "/Game/AnimalVarietyPack/Wolf/Animations/ANIM_Wolf_GetHitRight.ANIM_Wolf_GetHitRight")
        (set `self.Should Run?` true)
        (`KismetSystemLibrary.Delay` 0.7)
        (`self.Stop Animation`)
        (if (not (`self.Is Dead?`))
          (`self.Decide Next Action` true))))))

(event `self.ReceiveBeginPlay`
  (`self.Decide Next Action` false))

(event `Decide Next Action`
  (params (`SkipDelay?` :type Boolean))
  (if (not `SkipDelay?`)
    (`KismetSystemLibrary.Delay` (`KismetMathLibrary.RandomFloatInRange` 1.0 8.0)))
  (if (`self.Should Run?`)
    (`self.Run Away`)
    (elif (`self.Is Tired?`)
      _
      (elif (not (`self.Is Hungry?`))
        (`self.Random Roam`)
        (`self.Regen Health`)))))

(event `Regen Health`
  ;[1 1 1] Regen Health
  (if (and (< (`self.Health`) (`self.MaxHealth`)) (not (`self.Should Run?`)))
    (bind _output_get (set `self.Health` (`KismetMathLibrary.Clamp` (+ (`self.Health`) (`self.HealthGain`)) 0 (`self.MaxHealth`))))
    (if (not (== _output_get (`self.MaxHealth`)))
      (`KismetSystemLibrary.Delay` 1.0 :!label _label)
      (`self.Regen Health`))
    (else
      (goto _label))))

(event `Random Roam`
  ;[1 1 1] Random roam
  (set `CharacterMovementComponent.MaxWalkSpeed` 200.0 (`self.CharacterMovement`))
  (`|AIMoveTo` self (`NavigationSystemV1.K2_GetRandomReachablePointInRadius` (`self.K2_GetActorLocation`) 1500.0 null null) null
    (:`OnSuccess`
      (`self.Decide Next Action` false))))

(event `self.ReceiveHit`
  (params (MyComp :type "PrimitiveComponent Object Reference") (Other :type "Actor Object Reference") (OtherComp :type "PrimitiveComponent Object Reference") (bSelfMoved :type Boolean) (HitLocation :type "Vector Structure") (HitNormal :type "Vector Structure") (NormalImpulse :type "Vector Structure") (Hit :type "HitResult Structure (by ref)"))
  ;[1 1 1] Hit
  (bind _asbp_projectile (cast `/Game/Projectile/BP_Projectile` Other))
  (set `self.Damage` 50)
  (`self.Take Damage`)
  (`self.K2_DestroyActor` _asbp_projectile))

(event `Run Away`
  ;[1 1 1] Run away
  (set `CharacterMovementComponent.MaxWalkSpeed` 700.0 (`self.CharacterMovement`))
  (`|AIMoveTo` self (`NavigationSystemV1.K2_GetRandomReachablePointInRadius` (`self.K2_GetActorLocation`) (`KismetMathLibrary.RandomFloatInRange` 1000.0 3000.0) null null) null
    (:`OnSuccess`
      (`self.Decide Next Action` true))))

(fn `Play Animation`
  (params (Animation :type "AnimationAsset Object Reference") (`Should Loop?` :type Boolean)))

(fn `Stop Animation`)

(fn `UserConstructionScript`)